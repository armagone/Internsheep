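; Time manager that runs the in-game day clock, day count and end-of-day and end-of-game screens.
; Tick accumulates total playtime and advances in-game time by a GameSpeed multiplier, stopping when the ending hour is reached.
; Day end shows a random EventManager event on the HUD, and MoveToNextDay activates it and restarts the clock.
; The construction script creates the HUD and initializes EventManager and TaskManager.
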(event EventTick
  (params (DeltaSeconds :type Float%20%28single-precision%29))
  (TimeRelated|AddTimetoTimers DeltaSeconds)
  (bind _isover (TimeRelated|CheckifDayIsOver))
  (if _isover
    (Variables|Default|SetgameSpeed "NewEnumerator10")
    (HUDRelated|ChangetoEndOfDayHUD)))

(fn ConstructionScript
  (bind _self self)
  (CallFunction|Init)
  (Default|Init (Variables|Default|GetEventManager) _self)
  (Default|Init (Variables|Default|GetTaskManager) _self))

(fn SetGameSpeed
  (params (gameSped :type EGameSpeed%20Enum))
  (Variables|Default|SetgameSpeed gameSped))

(fn AddTimetoTimers
  (params (deltaTime :type Float%20%28single-precision%29))
  (Variables|Timers|SettotalPlaytimeTime (+ deltaTime (Variables|Timers|GettotalPlaytimeTime)))
  (bind _gamespeedfloat (Getters|GetGameSpeedFloat))
  (TimeRelated|AddTimetoIngameTimer deltaTime _gamespeedfloat))

(fn AddTimetoIngameTimer
  (params (deltaTime :type Float%20%28single-precision%29) (factor :type Float%20%28single-precision%29))
  (Variables|Timers|SetcurrentIngameTime (+ (* deltaTime factor) (Variables|Timers|GetcurrentIngameTime))))

(fn Load
  (params (totalPlaytimeTime :type Float%20%28single-precision%29) (currentIngameTime :type Float%20%28single-precision%29) (currentDayNumber :type Integer) (hourDurationInSeconds :type Float%20%28single-precision%29) (startingHour :type Float%20%28single-precision%29) (endingHour :type Float%20%28single-precision%29))
  (Variables|Timers|SettotalPlaytimeTime totalPlaytimeTime)
  (Variables|Timers|SetcurrentIngameTime currentIngameTime)
  (Variables|Default|SetcurrentDayNumber currentDayNumber)
  (Setters|SetHourDurationinSec hourDurationInSeconds)
  (Setters|SetDayDuration startingHour endingHour)
  (Variables|Default|SetgameSpeed "NewEnumerator10"))

(fn GetGameSpeed
  (return (Variables|Default|GetgameSpeed)))

(fn GetGameSpeedFloat
  (switch Utilities|FlowControl|Switch|SwitchonEGameSpeed (Variables|Default|GetgameSpeed)
    (:NewEnumerator10
      (return 0.0))
    (:NewEnumerator4
      (return 0.25))
    (:NewEnumerator6
      (return 0.5))
    (:NewEnumerator7
      (return 1.0))
    (:NewEnumerator8
      (return 2.0))
    (:NewEnumerator9
      (return 4.0))))

(fn GetTotalPlaytime
  (return (Variables|Timers|GettotalPlaytimeTime)))

(fn GetCurrentIngameTime
  (return (Variables|Timers|GetcurrentIngameTime)))

(fn CheckifDayIsOver
  (if (>= (Variables|Timers|GetcurrentIngameTime) (Variables|DayDurationRelated|GetdayEndingHourInSec))
    (return true)
    (else
      (return false))))

(fn SetDayDuration
  (params (startingHour :type Float%20%28single-precision%29) (endingHour :type Float%20%28single-precision%29))
  (bind _output_get (Variables|DayDurationRelated|SetdayStartingHour startingHour))
  (Variables|DayDurationRelated|SetdayStartingHourInSec (* _output_get (Variables|DayDurationRelated|GethourDurationInSec)))
  (bind _output_get_2 (Variables|DayDurationRelated|SetdayEndingHour endingHour))
  (Variables|DayDurationRelated|SetdayEndingHourInSec (* _output_get_2 (Variables|DayDurationRelated|GethourDurationInSec))))

(fn SetHourDurationinSec
  (params (hourDuration :type Float%20%28single-precision%29))
  (Setters|SetHourDurationinSec hourDuration)
  (Variables|DayDurationRelated|SetdayDurationInSec (* hourDuration 24.0)))

(fn MovetoNextDay
  (Math|Integer|IncrementInt (Variables|Default|GetcurrentDayNumber)
    (:%20%20
      (Variables|Timers|SetcurrentIngameTime (Variables|DayDurationRelated|GetdayStartingHourInSec))
      (Variables|Default|SetisDayOver false)
      (Setters|SetGameSpeed "NewEnumerator7")
      (Default|ActivateLastEventPicked (Variables|Default|GetEventManager)))))

(fn GetDurationinSec
  (params (days :type Float%20%28single-precision%29) (hours :type Float%20%28single-precision%29) (minutes :type Float%20%28single-precision%29) (seconds :type Float%20%28single-precision%29))
  (return (* (+ (* 24 days) hours (/ minutes 6e+01) (/ seconds 3.6e+03)) (Variables|DayDurationRelated|GethourDurationInSec))))

(fn GetCurrentDayNumber
  (return (Variables|Default|GetcurrentDayNumber)))

(fn GetDayStartingHour
  (return (Variables|DayDurationRelated|GetdayStartingHour)))

(fn GetDayEndingHour
  (return (Variables|DayDurationRelated|GetdayEndingHour)))

(fn Init
  (Setters|SetDayDuration (Variables|DayDurationRelated|GetdayStartingHour) (Variables|DayDurationRelated|GetdayEndingHour))
  (Variables|Timers|SetcurrentIngameTime (Variables|DayDurationRelated|GetdayStartingHourInSec))
  (bind _returnvalue (UserInterface|CreateWidget "/Game/MaximeBP/HUD/GameStateCustomHUD.GameStateCustomHUD_C"))
  (bind _output_get (Variables|Default|SethudWidget _returnvalue))
  (UserInterface|Viewport|AddtoViewport _output_get 0)
  (Default|Init (Variables|Default|GethudWidget)))

(fn ChangetoEndOfDayHUD
  (bind _hudwidget (Variables|Default|GethudWidget))
  (if (not (Variables|Default|GetisDayOver))
    (bind _eventdescription (Default|PickRandomEvent (Variables|Default|GetEventManager)))
    (LocalVariables|SeteventDescription _eventdescription)
    (Variables|/Game/MaximeBP/HUD/GameStateCustomHUD.GameStateCustomHUD_C|SetisHudActivated (Variables|Default|GethudWidget) true)
    (Variables|/Game/MaximeBP/HUD/GameStateCustomHUD.GameStateCustomHUD_C|SeteventDescription _hudwidget (LocalVariables|GeteventDescription))
    (Variables|/Game/MaximeBP/HUD/GameStateCustomHUD.GameStateCustomHUD_C|SetdayNumber _hudwidget (Variables|Default|GetcurrentDayNumber))
    (Variables|Default|SetisDayOver true)))

(fn GetCurrentIngameTimeText
  (bind _output_get (LocalVariables|Sethours (Math|Float|Truncate (/ (Variables|Timers|GetcurrentIngameTime) (Variables|DayDurationRelated|GethourDurationInSec)))))
  (LocalVariables|Setminutes (Math|Float|Truncate (* 60 (/ (- (Variables|Timers|GetcurrentIngameTime) (* _output_get (Variables|DayDurationRelated|GethourDurationInSec))) (Variables|DayDurationRelated|GethourDurationInSec)))))
  (return (Utilities|Text|FormatText "{hours}:{minutes}" (Utilities|Text|ToText(Integer) (LocalVariables|Gethours) true 2 2) (Utilities|Text|ToText(Integer) (LocalVariables|Getminutes) true 2 2))))

(fn ChangetoEndOfGameHUD
  (bind _hudwidget (Variables|Default|GethudWidget))
  (Setters|SetGameSpeed "NewEnumerator10")
  (LocalVariables|SeteventDescription "Nous avons terminé notre mission. 
Il est désormais temps de rentrer sur Terre ...")
  (Variables|/Game/MaximeBP/HUD/GameStateCustomHUD.GameStateCustomHUD_C|SetisHudActivated (Variables|Default|GethudWidget) true)
  (Variables|/Game/MaximeBP/HUD/GameStateCustomHUD.GameStateCustomHUD_C|SeteventDescription _hudwidget (LocalVariables|GeteventDescription))
  (Variables|/Game/MaximeBP/HUD/GameStateCustomHUD.GameStateCustomHUD_C|SetisGameOver _hudwidget true)
  (Variables|/Game/MaximeBP/HUD/GameStateCustomHUD.GameStateCustomHUD_C|SetdayNumber _hudwidget (Variables|Default|GetcurrentDayNumber)))