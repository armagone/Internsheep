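; Task manager that holds the game's objectives, by default one French-language task to create and upgrade gravitational rings.
; Init stores the GameState, builds the task list with ten-day durations converted by TimeManager, and makes the first task current.
; UpdateTaskProgression adds quantities to elements matching the action type, then calls TimeManager's end-of-game HUD once all are met, without advancing to another task.
; A helper also fetches the Ressources widget.
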(fn Init
  (params (gameState :type Game%20State%20Object%20Reference))
  (Variables|Default|SetgameState gameState)
  (Addfunctions|AddDefaultTasks)
  (Variables|Default|SetcurrentTask (Utilities|Array|Get(acopy) (Variables|Default|GettasksList))))

(fn AddCustomTask
  (params (name :type Text) (description :type Text) (elements :type Array%20of%20Custom%20Task%20Element%20Structures))
  (bind _astime_manager (Utilities|Casting|CastToTimeManager (Variables|Default|GetgameState)))
  (bind _durationinsec (Default|GetDurationinSec _astime_manager 1e+01 0.0 0.0 0.0))
  (Utilities|Array|AddUnique (Variables|Default|GettasksList) (Utilities|Struct|MakeCustomTask name description elements 0.0 _durationinsec)))

(fn AddDefaultTasks
  (Addfunctions|AddCustomTask "Ingénieur, créer moi un bon anneau gravitationnel !" "L'ingénieur doit s'occuper de créer un anneau gravitationnel performant. 
 
- Creer 1 anneau(x) gravitationnel(s) 
- Améliore 1 anneau(x) gravitationnel(s)" (Utilities|Array|MakeArray (Utilities|Struct|MakeCustomTaskElement "NewEnumerator8" 2.0) (Utilities|Struct|MakeCustomTaskElement "NewEnumerator9" 2.0))))

(fn GetResourcesWidget
  (bind _foundwidgets (Widget|GetAllWidgetsOfClass "/Game/Menu/Ressources.Ressources_C" true))
  (bind _asressources (Utilities|Casting|CastToRessources (Utilities|Array|Get(acopy) _foundwidgets)))
  (return _asressources))

(fn GetCurrentTask
  (return (Variables|Default|GetcurrentTask)))

(fn UpdateTaskProgression
  (params (action :type EActionType%20Enum) (quantity :type Float%20%28single-precision%29))
  (for (_array_element _array_index) (.elements (Utilities|Struct|BreakCustomTask (Variables|Default|GetcurrentTask)))
    (if (== action (.actionType (Utilities|Struct|BreakCustomTaskElement _array_element)))
      (Utilities|Array|SetArrayElem (.elements (Utilities|Struct|BreakCustomTask (Variables|Default|GetcurrentTask))) _array_index (Utilities|Struct|MakeCustomTaskElement (.actionType (Utilities|Struct|BreakCustomTaskElement _array_element)) (+ (.quantityDone (Utilities|Struct|BreakCustomTaskElement _array_element)) quantity) (.quantityNeeded (Utilities|Struct|BreakCustomTaskElement _array_element))))))
  (bind _isdone (Taskfunctions|CheckifTaskDone))
  (if _isdone
    (bind _astime_manager (Utilities|Casting|CastToTimeManager (Variables|Default|GetgameState)))
    (Default|ChangetoEndOfGameHUD _astime_manager)))

(fn CheckifTaskDone
  (for _array_element (.elements (Utilities|Struct|BreakCustomTask (Variables|Default|GetcurrentTask)))
    (if (not (>= (.quantityDone (Utilities|Struct|BreakCustomTaskElement _array_element)) (.quantityNeeded (Utilities|Struct|BreakCustomTaskElement _array_element))))
      (Math|Integer|IncrementInt (LocalVariables|GetunfinishedTasks))))
  (return (== (LocalVariables|GetunfinishedTasks) 0)))