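; EventManager holds a list of custom game events, such as a stock disappearance, and rolls whether one happens.
; PickRandomEvent tests EventProbability, stores a random event's index and returns its description, or a no-event text.
; Activating an event, given directly or as the last pick, applies each element's quantity to food or construction supply through the Ressources widget, found by class search.
; Init stores the GameState and registers the default event.
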(fn Init
  (params (gameState :type Game%20State%20Object%20Reference))
  (Variables|Default|SetgameState gameState)
  (Addfunctions|AddDefaultEvents))

(fn AddCustomEvent
  (params (name :type Text) (description :type Text) (elements :type Array%20of%20Custom%20Event%20Element%20Structures))
  (Utilities|Array|AddUnique (Variables|Default|GeteventsList) (Utilities|Struct|MakeCustomEvent name description elements)))

(fn CheckifEventHappened
  (return (<= (Math|Random|RandomFloat) (Variables|Default|GeteventProbability))))

(fn PickRandomEvent
  (bind _haseventhappened (Getters|CheckifEventHappened))
  (if _haseventhappened
    (bind _eventid (Getters|GetRandomEventId))
    (bind _output_get (Variables|Default|SetlastPickedEventId _eventid))
    (if (!= _output_get -1)
      (return (.description (Utilities|Struct|BreakCustomEvent (Utilities|Array|Get(acopy) (Variables|Default|GeteventsList) _eventid))))
      (else
        (return (Variables|Default|GetnoEventDescription))))
    (else
      (return (Variables|Default|GetnoEventDescription)))))

(fn AddDefaultEvents
  (Addfunctions|AddCustomEvent "Disparitions de Stock" "Damn ! Une partie du stock a disparu ! 
- 200 de Nourriture 
- 200 de Matériel de Construction " (Utilities|Array|MakeArray (Utilities|Struct|MakeCustomEventElement "NewEnumerator1" -2e+02) (Utilities|Struct|MakeCustomEventElement "NewEnumerator0" -2e+02))))

(fn ActivateEvent
  (params (event :type Custom%20Event%20Structure))
  (bind _resourceswidget (CallFunction|GetResourcesWidget))
  (LocalVariables|SetresourcesWidget _resourceswidget)
  (for _array_element (.elements (Utilities|Struct|BreakCustomEvent event))
    (LocalVariables|SetquantityDone (.quantityDone (Utilities|Struct|BreakCustomEventElement _array_element)))
    (switch Utilities|FlowControl|Switch|SwitchonEActionType (.actionType (Utilities|Struct|BreakCustomEventElement _array_element))
      (:NewEnumerator1
        (Default|AddConstructionSupply (LocalVariables|GetresourcesWidget) (LocalVariables|GetquantityDone)))
      (:NewEnumerator0
        (Default|AddFood (LocalVariables|GetresourcesWidget) (LocalVariables|GetquantityDone))))))

(fn GetRandomEventId
  (bind _output_get (LocalVariables|SeteventListSize (Utilities|Array|Length (Variables|Default|GeteventsList))))
  (if (>= _output_get 1)
    (return (Math|Random|RandomIntegerinRange 0 (- (LocalVariables|GeteventListSize) 1)))
    (else
      (return -1))))

(fn GetResourcesWidget
  (bind _foundwidgets (Widget|GetAllWidgetsOfClass "/Game/Menu/Ressources.Ressources_C" true))
  (bind _asressources (Utilities|Casting|CastToRessources (Utilities|Array|Get(acopy) _foundwidgets)))
  (return _asressources))

(fn ActivateLastEventPicked
  (if (!= (Variables|Default|GetlastPickedEventId) -1)
    (bind _resourceswidget (CallFunction|GetResourcesWidget))
    (LocalVariables|SetresourcesWidget _resourceswidget)
    (for _array_element (.elements (Utilities|Struct|BreakCustomEvent (Utilities|Array|Get(acopy) (Variables|Default|GeteventsList) (Variables|Default|GetlastPickedEventId))))
      (LocalVariables|SetquantityDone (.quantityDone (Utilities|Struct|BreakCustomEventElement _array_element)))
      (switch Utilities|FlowControl|Switch|SwitchonEActionType (.actionType (Utilities|Struct|BreakCustomEventElement _array_element))
        (:NewEnumerator1
          (Default|AddConstructionSupply (LocalVariables|GetresourcesWidget) (LocalVariables|GetquantityDone)))
        (:NewEnumerator0
          (Default|AddFood (LocalVariables|GetresourcesWidget) (LocalVariables|GetquantityDone)))))))